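; Lever actor that a pawn interacts with to trigger another selected actor.
; Each interaction forwards an interact message to SelectedActor, then a FlipFlop alternates playing and reversing a timeline.
; The timeline's update pitches the handle mesh and also adds a Keycard gameplay tag to the instigator's BobActionComponent active tags on every update.
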(event `BobGameplayInterface.Interact`
  (params (InstigatorPawn :type "Pawn Object Reference"))
  (message `BobGameplayInterface.Interact` (`self.SelectedActor`) InstigatorPawn)
  (`/Engine/EditorBlueprintResources/StandardMacros.FlipFlop`
    (:`A`
      (bind (_direction _newtrack_0) (`Timeline|Switch Rotation` :!label _label)
        (:`Update`
          (`SceneComponent.K2_SetRelativeRotation` (`self.HandleMesh`) (`KismetMathLibrary.MakeRotator` 0.0 _newtrack_0) false false)
          (`BlueprintGameplayTagLibrary.AddGameplayTag` (`BobActionComponent.ActiveGameplayTags` (`self.GetComponentByClass` InstigatorPawn "/Script/ActionRougelike.BobActionComponent")) (`self.Keycard`)))))
    (:`B`
      (goto _label :!via `Reverse`))))

(fn `UserConstructionScript`)