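; Player controller for the ActionRougelike game that sets up the main HUD and provides hotkeys for saving and loading.
; When play state begins on a local controller, it creates the UI_MainHUD widget, adds it to the viewport and switches input to game only.
; Hardcoded L and K key events call the BobGameModeBase save and load functions, with a printed confirmation only on save.
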(event `self.BlueprintBeginPlayingState`
  (if (`self.IsLocalController`)
    (bind _returnvalue (`|CreateWidget` "/Game/ActionRougelike/UserInterface/UI_MainHUD.UI_MainHUD_C")) ; MOVE TO CONTROLLER
    (`UserWidget.AddToViewport` _returnvalue 0)
    (`WidgetBlueprintLibrary.SetInputMode_GameOnly` self)))

(event `Key|L`
  (params (Key :type "Key Structure"))
  (:`Pressed`
    (bind _asbob_game_mode_base (cast `BobGameModeBase` (`GameplayStatics.GetGameMode`)))
    (`BobGameModeBase.WriteSaveGame` _asbob_game_mode_base)
    (`KismetSystemLibrary.PrintString` "World Saved!")))

(event `Key|K`
  (params (Key :type "Key Structure"))
  (:`Pressed`
    (bind _asbob_game_mode_base (cast `BobGameModeBase` (`GameplayStatics.GetGameMode`)))
    (`BobGameModeBase.ReadSaveGame` _asbob_game_mode_base)))

(fn `UserConstructionScript`)