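; Bonfire is an interactable save point that lights its flame and saves the world when used.
; Interact sets FireActive, then calls WriteSaveGame on BobGameModeBase, prints a confirmation and updates the flames.
; OnActorLoaded prints the FireActive state and reapplies it, activating the Flame component only when the fire is active.
; The OnRep handler for FireActive is empty.
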(event `Update Flames`
  ;[0 0 0] Update Flames
  (if (`self.bFireActive`)
    (`ActorComponent.Activate` (`self.Flame`) false)))

(event `BobGameplayInterface.Interact`
  (params (InstigatorPawn :type "Pawn Object Reference"))
  ;[0 0 0] On Interact
  (set `self.bFireActive` true)
  (bind _asbob_game_mode_base (cast `BobGameModeBase` (`GameplayStatics.GetGameMode`)))
  (`BobGameModeBase.WriteSaveGame` _asbob_game_mode_base)
  (`KismetSystemLibrary.PrintString` "World Saved!")
  (`self.Update Flames`))

(event `BobGameplayInterface.OnActorLoaded`
  ;[0 0 0] On Actor Loaded
  (`KismetSystemLibrary.PrintString` (`KismetStringLibrary.Conv_BoolToString` (`self.bFireActive`)))
  (`self.Update Flames`))

(fn `OnRep_bFireActive`)

(fn `UserConstructionScript`)