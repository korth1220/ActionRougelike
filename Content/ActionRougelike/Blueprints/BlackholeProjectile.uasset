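; Black hole projectile that destroys physics-simulating objects it touches and removes itself after a short lifetime.
; It calls Activate on its RadialForce component every Tick.
; Its collision sphere destroys any overlapping actor whose overlapped component simulates physics, and a timer started on BeginPlay destroys the projectile.
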(event `self.ReceiveBeginPlay`
  (`KismetSystemLibrary.K2_SetTimerDelegate` (delegate `DeleteHole`) 5.0))

(event `DeleteHole`
  (`self.K2_DestroyActor`))

(event `self.ReceiveTick`
  (params (DeltaSeconds :type "Float (single-precision)"))
  (`ActorComponent.Activate` (`self.RadialForce`) false))

(event `self.SphereCollision.OnComponentBeginOverlap`
  (params (OverlappedComponent :type "PrimitiveComponent Object Reference") (OtherActor :type "Actor Object Reference") (OtherComp :type "PrimitiveComponent Object Reference") (OtherBodyIndex :type Integer) (bFromSweep :type Boolean) (SweepResult :type "HitResult Structure (by ref)"))
  (`/Engine/EditorBlueprintResources/StandardMacros.IsValid` OtherActor
    (:`Is Valid`
      (if (`SceneComponent.IsSimulatingPhysics` OtherComp "None")
        (`self.K2_DestroyActor` OtherActor)))))

(fn `UserConstructionScript`)